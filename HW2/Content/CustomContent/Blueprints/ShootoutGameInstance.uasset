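; Game instance for the Shootout game that keeps the high score table and persists it through a SaveData save slot.
; SaveGameHandler loads the existing slot into HighScores, or creates a new save object and writes the current table.
; UpdateHighScores inserts Score above the first lower entry, drops the last to keep the list length fixed, then saves.
; HighScoreString concatenates the scores into one text value.
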(event Custom|SaveGameHandler
  (bind _returnvalue (SaveGame|DoesSaveGameExist (Variables|Default|GetSlot%20Name)))
  (if _returnvalue
    (bind _returnvalue_2 (SaveGame|LoadGamefromSlot (Variables|Default|GetSlot%20Name)))
    (bind _assave_data (Utilities|Casting|CastToSaveData _returnvalue_2))
    (Variables|Default|SetSave%20Data _assave_data)
    (CallFunction|LoadGameData)
    (else
      (bind _returnvalue_3 (SaveGame|CreateSaveGameObject "/Game/CustomContent/Blueprints/SaveData.SaveData_C"))
      (Variables|Default|SetSave%20Data _returnvalue_3)
      (CallFunction|SaveGameData))))

(fn UpdateHighScores
  (bind _highscores (Variables|Default|GetHighScores))
  (bind (_array_element _array_index) (Utilities|Array|ForEachLoopwithBreak _highscores :!label _label)
    (:LoopBody
      (if (> (Variables|Default|GetScore) _array_element)
        (Utilities|Array|Insert _highscores (Variables|Default|GetScore) _array_index)
        (Utilities|Array|RemoveIndex _highscores (Utilities|Array|LastIndex _highscores))
        (Variables|Default|SetScore 0)
        (goto _label Break)))
    (:Completed
      (CallFunction|SaveGameData)
      (return))))

(fn SaveGameData
  (bind _save_data (Variables|Default|GetSave%20Data))
  (Variables|/Game/CustomContent/Blueprints/SaveData.SaveData_C|SetHighScores _save_data (Variables|Default|GetHighScores))
  (SaveGame|SaveGametoSlot _save_data (Variables|Default|GetSlot%20Name))
  (return))

(fn LoadGameData
  (Variables|Default|SetHighScores (Variables|/Game/CustomContent/Blueprints/SaveData.SaveData_C|GetHighScores (Variables|Default|GetSave%20Data)))
  (return))

(fn HighScoreString
  (Variables|Default|SetScoreString "")
  (for _array_element (Variables|Default|GetHighScores)
    (Variables|Default|SetScoreString (Utilities|Text|ToText(String) (Utilities|String|Append (Utilities|String|ToString(Text) (Variables|Default|GetScoreString)) (Utilities|String|Append (Utilities|String|ToString(Integer) _array_element) " 
")))))
  (return (Variables|Default|GetScoreString)))