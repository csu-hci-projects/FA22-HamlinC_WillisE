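; Enemy pawn that carries a pistol and chases the player on sight.
; On BeginPlay it spawns an AIPistol and snaps it to the mesh's RevolverHoldPosition socket.
; PawnSensing flags whether the seen pawn is the player, then AIMoveTo closes in; FireAtPlayer is an empty stub.
; Mesh overlaps with Projectile-tagged actors play a sound, swap mesh materials and print a debug string, without applying damage.
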(event OnSeePawn(PawnSensing)
  (params (Pawn :type Pawn%20Object%20Reference))
  (Variables|Default|SetIs%20Seeing%20Player? (== Pawn (Game|Player|GetPlayerPawn 0)))
  (CallFunction|EnterPlayerRange))

(event OnComponentBeginOverlap(Mesh)
  (params (OverlappedComponent :type Primitive%20Component%20Object%20Reference) (OtherActor :type Actor%20Object%20Reference) (OtherComp :type Primitive%20Component%20Object%20Reference) (OtherBodyIndex :type Integer) (bFromSweep :type Boolean) (SweepResult :type Hit%20Result%20Structure%20%28by%20ref%29))
  (bind _mesh (Variables|Character|GetMesh))
  (if (Actor|ActorHasTag OtherActor "Projectile")
    (Audio|PlaySoundatLocation "/Engine/EditorSounds/Notifications/CompileFailed.CompileFailed" (Transformation|GetActorLocation) "0, 0, 0" 1.0 1.0 0.0 0 0 0 0)
    (for _index (range 0 4)
      (Utilities|IsValid _mesh
        (:Is%20Valid
          (Rendering|Material|SetMaterial _mesh _index "/Game/FPWeapon/Materials/M_FPGun.M_FPGun"))))
    (Development|PrintString "Hello")))

(event Custom|Enter%20Player%20Range
  (if (Variables|Default|GetIs%20Seeing%20Player?)
    (AI|AIMoveTo self "0, 0, 0" (Game|GetPlayerCharacter 0) 1.6e+02 false)))

(event Custom|FireAtPlayer)

(event EventBeginPlay
  (bind _returnvalue (Game|SpawnActorfromClass "/Game/CustomContent/Blueprints/AIPistol.AIPistol_C" (Transformation|GetSocketTransform (Variables|Character|GetMesh) "None" "RTS_World") "Undefined" 0 0))
  (Transformation|AttachComponentToComponent _returnvalue (Variables|Character|GetMesh) "RevolverHoldPosition" "SnapToTarget" "SnapToTarget" "SnapToTarget" true))

(event Collision|EventActorBeginOverlap
  (params (OtherActor :type Actor%20Object%20Reference)))

(event EventTick
  (params (DeltaSeconds :type Float%20%28single-precision%29)))

(fn ConstructionScript)