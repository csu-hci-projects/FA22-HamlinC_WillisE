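; Behavior Tree task that moves an Enemy pawn toward the player's location, sampled when the move starts.
; When the move succeeds or fails, it reads CanSeePlayer from the EnemyController and returns that as the task result.
; Seeing the player resets the acceptance radius, while losing sight halves it for later moves on the same task instance.
; Aborting finishes immediately without explicitly stopping the move.
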(event EventReceiveExecuteAI
  (params (OwnerController :type AI%20Controller%20Object%20Reference) (ControlledPawn :type Pawn%20Object%20Reference))
  (bind _asenemy (Utilities|Casting|CastToEnemy ControlledPawn))
  (AI|AIMoveTo _asenemy (Transformation|GetActorLocation (Game|Player|GetPlayerPawn 0)) 0 (Variables|Default|GetAcceptanceRadius) true
    (:OnSuccess
      _)
    (:OnFail
      _))
  (bind _asenemy_controller (Utilities|Casting|CastToEnemyController (Pawn|GetController _asenemy)))
  (if (Variables|/Game/CustomContent/Blueprints/EnemyController.EnemyController_C|GetCanSeePlayer _asenemy_controller)
    (Variables|Default|SetAcceptanceRadius 2e+02)
    (else
      (Variables|Default|SetAcceptanceRadius (/ (Variables|Default|GetAcceptanceRadius) 2.0))))
  (AI|BehaviorTree|FinishExecute (Variables|/Game/CustomContent/Blueprints/EnemyController.EnemyController_C|GetCanSeePlayer _asenemy_controller)))

(event EventReceiveAbortAI
  (params (OwnerController :type AI%20Controller%20Object%20Reference) (ControlledPawn :type Pawn%20Object%20Reference))
  (Class|BTTaskBlueprintBase|FinishAbort))