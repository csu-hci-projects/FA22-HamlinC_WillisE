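; GameStart is the start-menu Blueprint that launches a new session of the ball game.
; On BeginPlay it creates the StartMenu widget and adds it to the viewport.
; The StartGame input action opens Lvl1, then resets lives, difficulty, completed goals and elapsed time on BallGameInstance.
; It then calls LoadSaveSlot and LoadGameData on that instance, after the reset.
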(event EventBeginPlay
  (bind _returnvalue (UserInterface|CreateWidget "/Game/UI/StartMenu.StartMenu_C"))
  (UserInterface|Viewport|AddtoViewport _returnvalue 0))

(event Collision|EventActorBeginOverlap
  (params (OtherActor :type Actor%20Object%20Reference)))

(event EventTick
  (params (DeltaSeconds :type Float%20%28single-precision%29)))

(event Input|ActionEvents|InputActionStartGame
  (params (Key :type Key%20Structure :default "None"))
  (:Pressed
    (Game|OpenLevel(byObjectReference) "/Game/Maps/Lvl-1.Lvl-1")
    (bind _asball_game_instance (Utilities|Casting|CastToBallGameInstance (Game|GetGameInstance)))
    (Variables|/Game/Blueprints/BallGameInstance.BallGameInstance_C|SetPlayerLives _asball_game_instance 3)
    (Variables|/Game/Blueprints/BallGameInstance.BallGameInstance_C|SetDifficulty _asball_game_instance 2)
    (Variables|/Game/Blueprints/BallGameInstance.BallGameInstance_C|SetGoals%20Completed _asball_game_instance 0)
    (Variables|/Game/Blueprints/BallGameInstance.BallGameInstance_C|SetTimePassed _asball_game_instance 0)
    (Default|LoadSaveSlot _asball_game_instance)
    (Default|LoadGameData _asball_game_instance)))

(fn ConstructionScript)