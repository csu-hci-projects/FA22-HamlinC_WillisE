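; End-of-game actor for the ball game that records the time high score, shows the end menu and handles restarting.
; On BeginPlay, IsNewHighScore inserts the run's time into the game instance's ascending high-score list and drops the last entry.
; It then shows EndMenu, stops the timer, saves the scores and calls ScoresToString.
; StartGame input opens Lvl1 and resets the run state in BallGameInstance.
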(event EventBeginPlay
  (Utilities|IsNewHighScore
    (:Out
      (bind _returnvalue (UserInterface|CreateWidget "/Game/UI/EndMenu.EndMenu_C"))
      (UserInterface|Viewport|AddtoViewport _returnvalue 0)
      (bind _asball_game_instance (Utilities|Casting|CastToBallGameInstance (Game|GetGameInstance)))
      (Default|StopCounting _asball_game_instance)
      (Default|SaveGameData _asball_game_instance (Variables|/Game/Blueprints/BallGameInstance.BallGameInstance_C|GetTimeHighScores _asball_game_instance))
      (Default|ScorestoString _asball_game_instance))))

(event Collision|EventActorBeginOverlap
  (params (OtherActor :type Actor%20Object%20Reference)))

(event EventTick
  (params (DeltaSeconds :type Float%20%28single-precision%29)))

(event Input|ActionEvents|InputActionStartGame
  (params (Key :type Key%20Structure :default "None"))
  (:Pressed
    (Game|OpenLevel(byObjectReference) "/Game/Maps/Lvl-1.Lvl-1")
    (bind _asball_game_instance (Utilities|Casting|CastToBallGameInstance (Game|GetGameInstance)))
    (Variables|/Game/Blueprints/BallGameInstance.BallGameInstance_C|SetPlayerLives _asball_game_instance 3)
    (Variables|/Game/Blueprints/BallGameInstance.BallGameInstance_C|SetDifficulty _asball_game_instance 2)
    (Variables|/Game/Blueprints/BallGameInstance.BallGameInstance_C|SetGoals%20Completed _asball_game_instance 0)
    (Variables|/Game/Blueprints/BallGameInstance.BallGameInstance_C|SetTimePassed _asball_game_instance 0)))

(fn ConstructionScript)