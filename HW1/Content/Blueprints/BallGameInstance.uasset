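; BallGameInstance holds the ball game's session state: lives, difficulty, elapsed time and completed goals.
; Events adjust lives and difficulty within limits, with a lost life also lowering difficulty, and a looping one-second timer drives the time count.
; It loads or creates a GameData save object, writes and reads high scores through it, and joins them into display text.
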(event Custom|Add%20Lives
  (bind _playerlives (Variables|Default|GetPlayerLives))
  ;[1 1 1] Lives Handler
  (if (< _playerlives 3)
    (Math|Integer|IncrementInt _playerlives)))

(event Custom|Load%20Save%20Slot
  (bind _returnvalue (SaveGame|DoesSaveGameExist (Variables|Default|GetSave%20Slot%20Name)))
  (if _returnvalue
    (bind _returnvalue_2 (SaveGame|LoadGamefromSlot (Variables|Default|GetSave%20Slot%20Name)))
    (bind _asgame_data (Utilities|Casting|CastToGameData _returnvalue_2))
    (Variables|Default|SetGameData _asgame_data)
    (else
      (bind _returnvalue_3 (SaveGame|CreateSaveGameObject "/Game/Blueprints/GameData.GameData_C"))
      (Variables|Default|SetGameData _returnvalue_3))))

(event Custom|Start%20Counting
  ;[1 1 1] timer
  (Utilities|Time|SetTimerbyFunctionName 0 (Variables|Default|GetCountName) 1.0 true))

(event Custom|Decrease%20Diffculty
  (bind _difficulty (Variables|Default|GetDifficulty))
  ;[1 1 1] Difficulty Handler
  (if (> _difficulty 0)
    (Math|Integer|DecrementInt _difficulty)))

(event Custom|Count
  ;[1 1 1] timer
  (Math|Integer|IncrementInt (Variables|Default|GetTimePassed)))

(event Custom|Remove%20Lives
  ;[1 1 1] Lives Handler
  (Math|Integer|DecrementInt (Variables|Default|GetPlayerLives)
    (:%20%20
      (CallFunction|DecreaseDiffculty))))

(event Custom|Stop%20Counting
  ;[1 1 1] timer
  (Utilities|Time|ClearTimerbyFunctionName 0 (Variables|Default|GetCountName)))

(event Custom|Add%20To%20Goals
  (Math|Integer|IncrementInt (Variables|Default|GetGoals%20Completed)))

(event Custom|Increase%20Difficulty
  (bind _difficulty (Variables|Default|GetDifficulty))
  ;[1 1 1] Difficulty Handler
  (if (< _difficulty 2)
    (Math|Integer|IncrementInt _difficulty)))

(fn SaveGameData
  (params (Score :type Array%20of%20Integers))
  (bind _gamedata (Variables|Default|GetGameData))
  (Variables|/Game/Blueprints/GameData.GameData_C|SetScores _gamedata Score)
  (bind _returnvalue (SaveGame|SaveGametoSlot _gamedata (Variables|Default|GetSave%20Slot%20Name)))
  (Development|PrintString (Utilities|String|ToString(Boolean) _returnvalue)))

(fn LoadGameData
  (Variables|Default|SetTimeHighScores (Variables|/Game/Blueprints/GameData.GameData_C|GetScores (Variables|Default|GetGameData)))
  (return))

(fn ScorestoString
  (Variables|Default|SetScoreString "")
  (for _array_element (Variables|Default|GetTimeHighScores)
    (Variables|Default|SetScoreString (Utilities|String|Append (Variables|Default|GetScoreString) (Utilities|String|Append (Utilities|String|ToString(Integer) _array_element) " 
"))))
  (return (Utilities|Text|ToText(String) (Variables|Default|GetScoreString))))