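; Instakill boss hazard that kills the player's BP_Ball on contact.
; A timeline started on BeginPlay drives the Cube's relative location as a looping movement.
; When the player pawn overlaps the actor, it prints a debug string and plays a sound at the ball, then after a short delay sets the ball's health to a large negative value.
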(event Collision|EventActorBeginOverlap
  (params (OtherActor :type Actor%20Object%20Reference))
  ;[1 1 1] Damage
  (if (== OtherActor (Game|Player|GetPlayerPawn 0))
    (Development|PrintString "KILL")
    (bind _asbp_ball (Utilities|Casting|CastToBP_Ball (Game|Player|GetPlayerPawn 0)))
    (Audio|PlaySoundatLocation "/Game/SuperGrid/TutorialLevel/SoundEffects/PingBing.PingBing" (Transformation|GetActorLocation _asbp_ball) "0, 0, 0" 1.0 1.0 0.0 0 0 0 0)
    (Utilities|FlowControl|Delay 0.2)
    (Default|SetPlayerHealth _asbp_ball -1e+04)))

(event EventTick
  (params (DeltaSeconds :type Float%20%28single-precision%29)))

(event EventBeginPlay
  ;[1 1 1] looping movement
  (bind _newtrack_0 (Timeline|Timeline_0 Play)
    (:Update
      (Transformation|SetRelativeLocation (Variables|Default|GetCube) _newtrack_0 false false))))

(fn ConstructionScript)