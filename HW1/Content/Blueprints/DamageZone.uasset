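; Damage zone actor for the ball game that hurts the player while inside it, and destroys itself on BeginPlay unless Difficulty is above zero.
; Player overlap starts a looping, name-based timer that rechecks the overlap on each tick and clears itself once the ball leaves.
; Each tick inside passes DamageAmount scaled by Difficulty + 1 to BP_Ball's SetPlayerHealth and plays a ping at the ball.
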(event Custom|DamageTimer
  (bind _returnvalue (Game|Player|GetPlayerPawn 0))
  ;[1 1 1] DamageLogic
  (bind _asbp_ball (Utilities|Casting|CastToBP_Ball _returnvalue))
  (if (Collision|IsOverlappingActor _asbp_ball :!class /Script/Engine.Actor)
    (bind _asball_game_instance (Utilities|Casting|CastToBallGameInstance (Game|GetGameInstance)))
    (bind _asbp_ball_2 (Utilities|Casting|CastToBP_Ball _returnvalue))
    (Default|SetPlayerHealth _asbp_ball_2 (* (Variables|Default|GetDamageAmount) (+ (Variables|/Game/Blueprints/BallGameInstance.BallGameInstance_C|GetDifficulty _asball_game_instance) 1)))
    (Audio|PlaySoundatLocation "/Game/SuperGrid/TutorialLevel/SoundEffects/ShortPing.ShortPing" (Transformation|GetActorLocation _asbp_ball_2) "0, 0, 0" 1.0 1.0 0.0 0 0 0 0)
    (else
      (Utilities|Time|ClearTimerbyFunctionName 0 (Variables|Default|GetDamageTimerString)))))

(event EventBeginPlay
  (bind _asball_game_instance (Utilities|Casting|CastToBallGameInstance (Game|GetGameInstance)))
  (if (not (> (Variables|/Game/Blueprints/BallGameInstance.BallGameInstance_C|GetDifficulty _asball_game_instance) 0))
    (Actor|DestroyActor)))

(event Collision|EventActorBeginOverlap
  (params (OtherActor :type Actor%20Object%20Reference))
  (if (== OtherActor (Game|Player|GetPlayerPawn 0))
    (Development|PrintString "DAMAGE")
    (Utilities|Time|SetTimerbyFunctionName 0 (Variables|Default|GetDamageTimerString) 0.75 true)))

(event EventTick
  (params (DeltaSeconds :type Float%20%28single-precision%29)))

(fn ConstructionScript)